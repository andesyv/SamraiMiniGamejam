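; Player controller Blueprint for a first-person character that handles melee attack input and discarding the equipped weapon.
; On BeginPlay it sets game-only input, hides the cursor and caches the pawn as the player character.
; Attack plays the equipped weapon's data-defined montage on the first-person mesh unless a montage is already playing.
; Q destroys and clears the equipped weapon; an unconnected blade block montage branch never runs.
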(event EventBeginPlay
  (Input|SetInputModeGameOnly self)
  (Variables|Default|SetbShowMouseCursor false)
  (bind _asfirst_person_character (Utilities|Casting|CastToFirstPersonCharacter (Pawn|GetControlledPawn)))
  (Variables|Default|SetPlayerCharacter _asfirst_person_character))

(event Input|ActionEvents|InputActionAttack
  (params (Key :type Key%20Structure))
  (bind _returnvalue (Pawn|GetControlledPawn))
  (bind _playercharacter (Variables|Default|GetPlayerCharacter))
  (bind _asfirst_person_character (Utilities|Casting|CastToFirstPersonCharacter _returnvalue))
  (bind _equippedweapon (Variables|/Game/Blueprint/FirstPersonCharacter.FirstPersonCharacter_C|Getequippedweapon _playercharacter))
  (bind _returnvalue_2 (Class|SamraiMiniGamejamCharacter|GetMesh1P _asfirst_person_character))
  (:Pressed
    (if (not (Class|AnimInstance|IsAnyMontagePlaying (Components|SkeletalMesh|GetAnimInstance _returnvalue_2)))
      (Utilities|IsValid _equippedweapon
        (:Is%20Valid
          (Animation|Montage|PlayMontage _returnvalue_2 (Variables|/Script/SamraiMiniGamejam.WeaponData|GetAttackAnimation (Variables|/Game/BP_Weapon.BP_Weapon_C|Getweapondata _equippedweapon))))))))

(event Input|ActionEvents|InputActionBlock
  (params (Key :type Key%20Structure)))

(event Input|KeyboardEvents|Q
  (params (Key :type Key%20Structure))
  (bind _playercharacter (Variables|Default|GetPlayerCharacter))
  (:Pressed
    (Utilities|IsValid (Variables|/Game/Blueprint/FirstPersonCharacter.FirstPersonCharacter_C|Getequippedweapon _playercharacter)
      (:Is%20Valid
        (Actor|DestroyActor (Variables|/Game/Blueprint/FirstPersonCharacter.FirstPersonCharacter_C|Getequippedweapon _playercharacter))
        (Variables|/Game/Blueprint/FirstPersonCharacter.FirstPersonCharacter_C|Setequippedweapon _playercharacter 0)))))

(fn ConstructionScript)